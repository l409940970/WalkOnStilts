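; Physics-driven player that walks by manually lifting and swinging two constrained legs under a body.
; Mouse buttons raise each leg through timelines driving its constraint's linear Z drive and limit; axis input steps lifted legs with impulses at scene-component locations.
; Body input adds forward impulses, alongside a constant push each Tick.
; Tick also measures lean from the feet midpoint, easing body rotation to zero upon returning within 10 degrees of upright.
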(event Custom|LiftRIght
  (params (isLift :type Boolean))
  (bind _physicsconstraintright (Variables|Default|GetPhysicsConstraintRight))
  ;[1 1 1] 抬腿
  (bind _output_get (Variables|Default|SetisLiftRight isLift))
  (if _output_get
    (bind _newtrack_0 (Timeline|Timeline_Right Play)
      (:Update
        (Class|PhysicsConstraintComponent|SetLinearDriveParams _physicsconstraintright (Math|Float|Lerp 0.0 (Variables|Default|GetPositionStrength) _newtrack_0) 0.0 0.0)
        (Class|PhysicsConstraintComponent|SetLinearZLimit _physicsconstraintright "LCM_Limited" (Math|Float|Absolute(Float) (Math|Float|Lerp 0.0 (Variables|Default|GetLimitSize) _newtrack_0)))
        (Class|PhysicsConstraintComponent|SetLinearPositionTarget _physicsconstraintright (Math|Vector|MakeVector 0.0 0.0 (Math|Float|Lerp 0.0 (Variables|Default|GetLimitSize) _newtrack_0)))))
    (else
      (Timeline|Timeline_Right Reverse))))

(event Custom|LIftLeft
  (params (isLift :type Boolean))
  (bind _physicsconstraintleft (Variables|Default|GetPhysicsConstraintLeft))
  ;[1 1 1] 抬腿
  (bind _output_get (Variables|Default|SetisLiftLeft isLift))
  (if _output_get
    (bind _newtrack_0 (Timeline|Timeline_Left Play)
      (:Update
        (Class|PhysicsConstraintComponent|SetLinearDriveParams _physicsconstraintleft (Math|Float|Lerp 0.0 (Variables|Default|GetPositionStrength) _newtrack_0) 0.0 0.0)
        (Class|PhysicsConstraintComponent|SetLinearZLimit _physicsconstraintleft "LCM_Limited" (Math|Float|Absolute(Float) (Math|Float|Lerp 0.0 (Variables|Default|GetLimitSize) _newtrack_0)))
        (Class|PhysicsConstraintComponent|SetLinearPositionTarget _physicsconstraintleft (Math|Vector|MakeVector 0.0 0.0 (Math|Float|Lerp 0.0 (Variables|Default|GetLimitSize) _newtrack_0)))))
    (else
      (Timeline|Timeline_Left Reverse))))

(event Custom|Recover
  (CallFunction|MoveBody (Variables|Default|GetInitForceValue))
  (bind _vector (CallFunction|ReturnCenter))
  (if (<= (Class|KismetMathLibrary|DegAcos (Math|Vector|DotProduct _vector "0, 0,1.000000")) 1e+01)
    (if (and (Variables|Default|GetisRecover) (not (Audio|Components|Audio|IsPlaying (Variables|Default|GetTimeline_SetRot))))
      (Variables|Default|SetisRecover false)
      (Variables|Default|SetInitRot (Transformation|GetWorldRotation (Variables|Default|GetBody)))
      (bind _newtrack_0 (Timeline|Timeline_SetRot PlayFromStart)
        (:Update
          (Transformation|SetWorldRotation (Variables|Default|GetBody) (Math|Rotator|Lerp(Rotator) (Variables|Default|GetInitRot) "0, 0, 0" _newtrack_0) false false))))
    (else
      (Variables|Default|SetisRecover true))))

(event EventBeginPlay
  (CallFunction|Init))

(event EventTick
  (params (DeltaSeconds :type Float%20%28single-precision%29))
  (CallFunction|Recover))

(event Input|ActionEvents|InputActionLeftMousePress
  (params (Key :type Key%20Structure :default "None"))
  (:Pressed
    (CallFunction|LIftLeft true))
  (:Released
    (CallFunction|LIftLeft false)))

(event Input|ActionEvents|InputActionRightMousePress
  (params (Key :type Key%20Structure :default "None"))
  (:Pressed
    (CallFunction|LiftRIght true))
  (:Released
    (CallFunction|LiftRIght false)))

(event Input|AxisEvents|InputAxisMoveBody
  (params (AxisValue :type Float%20%28single-precision%29))
  (CallFunction|MoveBody (* AxisValue (* (Utilities|Time|GetWorldDeltaSeconds) 1.2e+02))))

(event Input|AxisEvents|InputAxisMoveLeft
  (params (AxisValue :type Float%20%28single-precision%29))
  (if (and (Variables|Default|GetisLiftLeft) (!= AxisValue 0.0))
    (CallFunction|Step (Math|Float|SelectFloat 1.0 -1.0 (> AxisValue 0.0)) true)))

(event Input|AxisEvents|InputAxisMoveRight
  (params (AxisValue :type Float%20%28single-precision%29))
  (if (and (Variables|Default|GetisLiftRight) (!= AxisValue 0.0))
    (CallFunction|Step (Math|Float|SelectFloat 1.0 -1.0 (> AxisValue 0.0)) false)))

(fn ConstructionScript)

(fn BPMoveBody
  (params (value :type Float%20%28single-precision%29))
  (Physics|AddImpulse (Variables|Default|GetBody) (* (* (Math|Vector|GetForwardVector (Variables|Default|GetBody)) value) (Variables|Default|GetMoveBodyValue)) "None" false))

(fn BPStep
  (params (value :type Float%20%28single-precision%29) (isLeft :type Boolean))
  (bind _rightleg (Variables|Default|GetRIghtLeg))
  (bind _stepvalue (Variables|Default|GetStepValue))
  (bind _leftleg (Variables|Default|GetLeftLeg))
  (bind _returnvalue (* value _stepvalue))
  (bind _returnvalue_2 (select isLeft _leftleg _rightleg))
  (bind _returnvalue_3 (Math|Vector|GetForwardVector _returnvalue_2))
  (bind _returnvalue_4 (* _returnvalue_3 _returnvalue))
  (Physics|AddImpulseatLocation _returnvalue_2 _returnvalue_4 (Transformation|GetWorldLocation (select isLeft (Variables|Default|GetLeftScene) (Variables|Default|GetRightScene))) "None")
  (Development|PrintString (Utilities|String|ToString(Vector) _returnvalue_4)))

(fn BPInit
  (Class|PhysicsConstraintComponent|SetAngularSwing2Limit (Variables|Default|GetPhysicsConstraintRight) "ACM_Limited" 4e+01))

(fn BPReturnCenter
  (bind _leftscene (Variables|Default|GetLeftScene))
  (bind _rightscene (Variables|Default|GetRightScene))
  (bind _returnvalue (Transformation|GetWorldLocation _rightscene))
  (bind _returnvalue_2 (Transformation|GetWorldLocation _leftscene))
  (return (Math|Vector|GetUnitDirection(Vector) (Math|Vector|MakeVector (/ (+ (.x _returnvalue_2) (.x _returnvalue)) 2.0) (/ (+ (.y _returnvalue_2) (.y _returnvalue)) 2.0) (Math|Float|Min(Float) (.z _returnvalue_2) (.z _returnvalue))) (Transformation|GetWorldLocation (Variables|Default|GetBodyScene)))))